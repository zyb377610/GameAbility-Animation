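; BP_GASCharacter is a character Blueprint that handles basic player movement and camera look from axis inputs.
; MoveForward and MoveRight add movement along the actor's forward and right vectors, while Turn and LookUp add controller yaw and pitch.
; Each input reaches the pawn through CharacterMovement's GetPawnOwner, and Turn also prints its axis value.
; Despite the GAS name, the graphs contain no ability system logic.
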(event EventBeginPlay)

(event Collision|EventActorBeginOverlap
  (params (OtherActor :type Actor%20Object%20Reference)))

(event EventTick
  (params (DeltaSeconds :type Float%20%28single-precision%29)))

(event Input|AxisEvents|InputAxisMoveForward
  (params (AxisValue :type Float%20%28single-precision%29))
  (Pawn|Input|AddMovementInput (Class|PawnMovementComponent|GetPawnOwner (Variables|Character|GetCharacterMovement)) (Transformation|GetActorForwardVector) AxisValue false))

(event Input|AxisEvents|InputAxisTurn
  (params (AxisValue :type Float%20%28single-precision%29))
  (Pawn|Input|AddControllerYawInput (Class|PawnMovementComponent|GetPawnOwner (Variables|Character|GetCharacterMovement)) AxisValue)
  (Development|PrintString (Utilities|String|ToString(Float) AxisValue)))

(event Input|AxisEvents|InputAxisMoveRight
  (params (AxisValue :type Float%20%28single-precision%29))
  (Pawn|Input|AddMovementInput (Class|PawnMovementComponent|GetPawnOwner (Variables|Character|GetCharacterMovement)) (Transformation|GetActorRightVector) AxisValue false))

(event Input|AxisEvents|InputAxisLookUp
  (params (AxisValue :type Float%20%28single-precision%29))
  (Pawn|Input|AddControllerPitchInput (Class|PawnMovementComponent|GetPawnOwner (Variables|Character|GetCharacterMovement)) AxisValue))

(fn ConstructionScript)